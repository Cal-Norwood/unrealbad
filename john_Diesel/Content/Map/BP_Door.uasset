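; BP_Door is a map door that slides up to open and back down to its origin to close.
; OpenDoor and closedoor events each restart their own timeline, which moves the Door component's relative location without sweeping.
; Each update lerps from the door's current location rather than a stored start, so motion compounds instead of tracking the curve directly.
; Neither event stops the other timeline, and nothing in this Blueprint triggers them.
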(event Custom|Open%20Door
  (bind _door (Variables|Default|GetDoor))
  ;[1 1 1] Door Open
  (bind _newtrack_0 (Timeline|Opening PlayFromStart)
    (:Update
      (Transformation|SetRelativeLocation _door (Math|Vector|Lerp(Vector) (Variables|/Script/Engine.SceneComponent|GetRelativeLocation _door) "0.000000,0.000000,260.000000" _newtrack_0) false false))))

(event Custom|close%20door
  (bind _door (Variables|Default|GetDoor))
  ;[1 1 1] Door Close
  (bind _newtrack_0 (Timeline|Timeline PlayFromStart)
    (:Update
      (Transformation|SetRelativeLocation _door (Math|Vector|Lerp(Vector) (Variables|/Script/Engine.SceneComponent|GetRelativeLocation _door) "0.000000,0.000000,0.000000" _newtrack_0) false false))))

(fn ConstructionScript)