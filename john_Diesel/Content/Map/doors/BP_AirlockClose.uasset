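; BP_AirlockClose is an airlock switch that alternately closes and opens its Door when interacted with, provided the player has no nozzle equipped.
; A FlipFlop drives the door and sets AirlockIsSealed on BP_AirlockOpen to match.
; A DoorDelay flag with a short delay blocks repeat presses, and the switch swaps material as feedback.
; A box overlap shows and hides a widget.
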(event OnComponentBeginOverlap(Box)
  (params (OverlappedComponent :type Primitive%20Component%20Object%20Reference) (OtherActor :type Actor%20Object%20Reference) (OtherComp :type Primitive%20Component%20Object%20Reference) (OtherBodyIndex :type Integer) (bFromSweep :type Boolean) (SweepResult :type Hit%20Result%20Structure%20%28by%20ref%29))
  (Rendering|SetVisibility (Variables|Default|GetWidget) true false))

(event OnComponentEndOverlap(Box)
  (params (OverlappedComponent :type Primitive%20Component%20Object%20Reference) (OtherActor :type Actor%20Object%20Reference) (OtherComp :type Primitive%20Component%20Object%20Reference) (OtherBodyIndex :type Integer))
  (Rendering|SetVisibility (Variables|Default|GetWidget) false false))

(event EventInteract
  (bind _door (Variables|Default|GetDoor))
  (bind _returnvalue (Actor|GetActorOfClass "/Game/FirstPerson/Blueprints/BP_FirstPersonCharacter.BP_FirstPersonCharacter_C"))
  (if (Variables|/Game/FirstPerson/Blueprints/BP_FirstPersonCharacter.BP_FirstPersonCharacter_C|GetNozzle%20Equipped _returnvalue)
    (Development|PrintString "Has Nozzle")
    (else
      (Development|PrintString "Doesnt have nozzle")
      (if (Variables|Default|GetDoor%20Delay)
        (Variables|Default|SetDoor%20Delay false)
        (Rendering|Material|SetMaterial (Variables|Default|GetSwitch) 0 "/AnimationSharing/AnimSharingGreen.AnimSharingGreen")
        (Utilities|FlowControl|FlipFlop
          (:A
            (Default|CloseDoor _door)
            (bind _returnvalue_2 (Actor|GetActorOfClass "/Game/Map/doors/airlock/BP_AirlockOpen.BP_AirlockOpen_C"))
            (Variables|/Game/Map/doors/airlock/BP_AirlockOpen.BP_AirlockOpen_C|SetAirlockIsSealed _returnvalue_2 true)
            (Utilities|FlowControl|Delay 2.0)
            (Variables|Default|SetDoor%20Delay true))
          (:B
            (Default|OpenDoor _door)
            (Variables|/Game/Map/doors/airlock/BP_AirlockOpen.BP_AirlockOpen_C|SetAirlockIsSealed _returnvalue_2 false)
            (Utilities|FlowControl|Delay 2.0)
            (Variables|Default|SetDoor%20Delay true)))
        (Rendering|Material|SetMaterial (Variables|Default|GetSwitch) 0 "/Engine/MapTemplates/Materials/BasicAsset01.BasicAsset01")))))

(fn ConstructionScript)