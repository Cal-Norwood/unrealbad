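; Airlock control actor that shows a widget while something overlaps its box and toggles the airlock door on Interact.
; Interaction requires a sealed airlock and the player's equipped nozzle, otherwise printing a hint.
; A FlipFlop alternates opening and closing the door, mirroring the state to BP_Gas_Gun's AirlockOpen flag.
; A DoorDelay gate with a short Delay blocks repeated presses, and the cube's material swaps as feedback.
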(event OnComponentBeginOverlap(Box)
  (params (OverlappedComponent :type Primitive%20Component%20Object%20Reference) (OtherActor :type Actor%20Object%20Reference) (OtherComp :type Primitive%20Component%20Object%20Reference) (OtherBodyIndex :type Integer) (bFromSweep :type Boolean) (SweepResult :type Hit%20Result%20Structure%20%28by%20ref%29))
  (Rendering|SetVisibility (Variables|Default|GetWidget) true false))

(event OnComponentEndOverlap(Box)
  (params (OverlappedComponent :type Primitive%20Component%20Object%20Reference) (OtherActor :type Actor%20Object%20Reference) (OtherComp :type Primitive%20Component%20Object%20Reference) (OtherBodyIndex :type Integer))
  (Rendering|SetVisibility (Variables|Default|GetWidget) false false))

(event EventInteract
  (bind _airlockdoor (Variables|Default|GetAirlockDoor))
  (if (Variables|Default|GetAirlockIsSealed)
    (bind _returnvalue (Actor|GetActorOfClass "/Game/FirstPerson/Blueprints/BP_FirstPersonCharacter.BP_FirstPersonCharacter_C"))
    (if (Variables|Default|GetDoor%20Delay)
      (Variables|Default|SetDoor%20Delay false)
      (if (Variables|/Game/FirstPerson/Blueprints/BP_FirstPersonCharacter.BP_FirstPersonCharacter_C|GetNozzle%20Equipped _returnvalue)
        (Rendering|Material|SetMaterial (Variables|Default|GetCube) 0 "/AnimationSharing/AnimSharingGreen.AnimSharingGreen")
        (Utilities|FlowControl|FlipFlop
          (:A
            (bind _returnvalue_2 (Actor|GetActorOfClass "/Game/Equipment/Fuel_Nozzle/BP_Gas_Gun.BP_Gas_Gun_C"))
            (Variables|/Game/Equipment/Fuel_Nozzle/BP_Gas_Gun.BP_Gas_Gun_C|SetAirlockOpen _returnvalue_2 true)
            (Default|OpenDoor _airlockdoor)
            (Utilities|FlowControl|Delay 2.0)
            (Variables|Default|SetDoor%20Delay true))
          (:B
            (bind _returnvalue_3 (Actor|GetActorOfClass "/Game/Equipment/Fuel_Nozzle/BP_Gas_Gun.BP_Gas_Gun_C"))
            (Variables|/Game/Equipment/Fuel_Nozzle/BP_Gas_Gun.BP_Gas_Gun_C|SetAirlockOpen _returnvalue_3 false)
            (Default|CloseDoor _airlockdoor)
            (Utilities|FlowControl|Delay 2.0)
            (Variables|Default|SetDoor%20Delay true)))
        (Rendering|Material|SetMaterial (Variables|Default|GetCube) 0 "/Engine/MapTemplates/Materials/BasicAsset01.BasicAsset01")
        (else
          (Development|PrintString "Pick up pump")
          (Variables|Default|SetDoor%20Delay true))))
    (else
      (Development|PrintString "seal airlock"))))

(fn ConstructionScript)