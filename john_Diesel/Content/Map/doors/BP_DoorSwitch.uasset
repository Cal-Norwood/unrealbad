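; BP_DoorSwitch is an interactable switch that alternately opens and closes a linked door.
; Interact runs a FlipFlop between the door's OpenDoor and CloseDoor calls, with the DoorDelay flag and a short Delay blocking repeat presses.
; The switch material turns green during the cooldown, then changes back.
; A box overlap shows and hides a widget.
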(event OnComponentBeginOverlap(Box)
  (params (OverlappedComponent :type Primitive%20Component%20Object%20Reference) (OtherActor :type Actor%20Object%20Reference) (OtherComp :type Primitive%20Component%20Object%20Reference) (OtherBodyIndex :type Integer) (bFromSweep :type Boolean) (SweepResult :type Hit%20Result%20Structure%20%28by%20ref%29))
  (Rendering|SetVisibility (Variables|Default|GetWidget) true false))

(event OnComponentEndOverlap(Box)
  (params (OverlappedComponent :type Primitive%20Component%20Object%20Reference) (OtherActor :type Actor%20Object%20Reference) (OtherComp :type Primitive%20Component%20Object%20Reference) (OtherBodyIndex :type Integer))
  (Rendering|SetVisibility (Variables|Default|GetWidget) false false))

(event EventInteract
  (bind _door (Variables|Default|GetDoor))
  (if (Variables|Default|GetDoor%20Delay)
    (Variables|Default|SetDoor%20Delay false)
    (Rendering|Material|SetMaterial (Variables|Default|GetSwitch) 0 "/AnimationSharing/AnimSharingGreen.AnimSharingGreen")
    (Utilities|FlowControl|FlipFlop
      (:A
        (Default|OpenDoor _door)
        (Utilities|FlowControl|Delay 2.0)
        (Variables|Default|SetDoor%20Delay true))
      (:B
        (Default|CloseDoor _door)
        (Utilities|FlowControl|Delay 2.0)
        (Variables|Default|SetDoor%20Delay true)))
    (Rendering|Material|SetMaterial (Variables|Default|GetSwitch) 0 "/Engine/MapTemplates/Materials/BasicAsset01.BasicAsset01")))

(fn ConstructionScript)